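; BP_KillZone is a trigger volume that sends the player back to a respawn point on contact.
; When the player character overlaps its Box, it reads the checkpoint state from BP_ThirdPersonGameMode.
; It teleports the character to the saved CheckpointTransform if one exists, otherwise to the "CrumblingStart" player start, setting both location and rotation.
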(event OnComponentBeginOverlap(Box)
  (params (OverlappedComponent :type Primitive%20Component%20Object%20Reference) (OtherActor :type Actor%20Object%20Reference) (OtherComp :type Primitive%20Component%20Object%20Reference) (OtherBodyIndex :type Integer) (bFromSweep :type Boolean) (SweepResult :type Hit%20Result%20Structure%20%28by%20ref%29))
  (if (== OtherActor (Game|GetPlayerCharacter 0))
    (bind _asbp_third_person_character (Utilities|Casting|CastToBP_ThirdPersonCharacter OtherActor)) ; Player
    (bind _asbp_third_person_game_mode (Utilities|Casting|CastToBP_ThirdPersonGameMode (Game|GetGameMode))) ; GM
    (Transformation|SetActorLocationAndRotation _asbp_third_person_character (.location (Math|Transform|SelectTransform (Variables|/Game/ThirdPerson/Blueprints/BP_ThirdPersonGameMode.BP_ThirdPersonGameMode_C|GetCheckpointTransform _asbp_third_person_game_mode) (Transformation|GetActorTransform (Class|GameModeBase|FindPlayerStart _asbp_third_person_game_mode (Pawn|GetController _asbp_third_person_character) "CrumblingStart")) (Variables|/Game/ThirdPerson/Blueprints/BP_ThirdPersonGameMode.BP_ThirdPersonGameMode_C|GetHasCheckpoint _asbp_third_person_game_mode))) (.rotation (Math|Transform|SelectTransform (Variables|/Game/ThirdPerson/Blueprints/BP_ThirdPersonGameMode.BP_ThirdPersonGameMode_C|GetCheckpointTransform _asbp_third_person_game_mode) (Transformation|GetActorTransform (Class|GameModeBase|FindPlayerStart _asbp_third_person_game_mode (Pawn|GetController _asbp_third_person_character) "CrumblingStart")) (Variables|/Game/ThirdPerson/Blueprints/BP_ThirdPersonGameMode.BP_ThirdPersonGameMode_C|GetHasCheckpoint _asbp_third_person_game_mode))) false true)))

(event EventBeginPlay)

(event Collision|EventActorBeginOverlap
  (params (OtherActor :type Actor%20Object%20Reference)))

(event EventTick
  (params (DeltaSeconds :type Float%20%28single-precision%29)))

(fn ConstructionScript)