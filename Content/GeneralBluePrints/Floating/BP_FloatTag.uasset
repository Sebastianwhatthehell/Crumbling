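; Actor component that makes tagged scene components on its owner bob up and down.
; On BeginPlay it gathers components matching TagName and stores each one's relative location with a random phase.
; Each tick it sets their relative Z to the stored location plus a sine offset driven by accumulated time, Speed and Amplitude, so they float out of sync.
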(event EventTick
  (params (DeltaSeconds :type Float%20%28single-precision%29))
  (Variables|Default|SetTime (+ DeltaSeconds (Variables|Default|GetTime)))
  (for _index (range 0 (- (Utilities|Array|Length (Variables|Default|GetComponents)) 1))
    (Transformation|SetRelativeLocation (Utilities|Array|Get(acopy) (Variables|Default|GetComponents) _index) (+ (Math|Vector|MakeVector 0.0 0.0 (* (Math|Trig|Sin(Radians) (+ (* (Variables|Default|GetTime) (Variables|Default|GetSpeed)) (Utilities|Array|Get(acopy) (Variables|Default|GetPhases) _index))) (Variables|Default|GetAmplitude))) (Utilities|Array|Get(acopy) (Variables|Default|GetInitialRelLocs) _index)) false false)))

(event EventBeginPlay
  (for (_array_element _array_index) (Actor|GetComponentsbyTag (Components|GetOwner) "/Script/Engine.SceneComponent" (Variables|Default|GetTagName))
    (Utilities|Array|SetArrayElem (Variables|Default|GetComponents) _array_index _array_element true)
    (Utilities|Array|SetArrayElem (Variables|Default|GetInitialRelLocs) _array_index (Variables|/Script/Engine.SceneComponent|GetRelativeLocation _array_element) true)
    (Utilities|Array|SetArrayElem (Variables|Default|GetPhases) _array_index (Math|Random|RandomFloatinRange 0.0 6.283185) true)))