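; BP_PuzzleTrigger is a puzzle trigger volume that reacts to overlapping actors tagged PuzzleTrigger.
; Begin overlap updates a per-actor count map and, on a zero-count check, sets IsTriggered, lights TargetImage's glow and registers activation with ConnectedCover.
; End overlap removes the actor's entry outright, and an empty map clears the flag and glow and registers deactivation with the cover.
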(event OnComponentBeginOverlap(TriggerBox)
  (params (OverlappedComponent :type Primitive%20Component%20Object%20Reference) (OtherActor :type Actor%20Object%20Reference) (OtherComp :type Primitive%20Component%20Object%20Reference) (OtherBodyIndex :type Integer) (bFromSweep :type Boolean) (SweepResult :type Hit%20Result%20Structure%20%28by%20ref%29))
  (bind _overlapcounts (Variables|Default|GetOverlapCounts))
  (bind (_value _returnvalue) (Utilities|Map|Find _overlapcounts OtherActor))
  (bind _returnvalue_2 (select _returnvalue 0 _value))
  (if (Actor|ActorHasTag OtherActor "PuzzleTrigger")
    (Utilities|Map|Add (Variables|Default|GetOverlapCounts) OtherActor (+ _returnvalue_2 1))
    (if (== _returnvalue_2 0)
      (Variables|Default|SetIsTriggered true)
      (Default|ActivateGlow (Variables|Default|GetTargetImage) 5.0)
      (Default|RegisterTriggerActivated (Variables|Default|GetConnectedCover)))))

(event OnComponentEndOverlap(TriggerBox)
  (params (OverlappedComponent :type Primitive%20Component%20Object%20Reference) (OtherActor :type Actor%20Object%20Reference) (OtherComp :type Primitive%20Component%20Object%20Reference) (OtherBodyIndex :type Integer))
  (bind _overlapcounts (Variables|Default|GetOverlapCounts))
  (if (Actor|ActorHasTag OtherActor "PuzzleTrigger")
    (if (.ReturnValue (Utilities|Map|Find (Variables|Default|GetOverlapCounts) OtherActor))
      (Utilities|Map|Remove _overlapcounts OtherActor)
      (if (== (Utilities|Map|Length _overlapcounts) 0)
        (Variables|Default|SetIsTriggered false)
        (Default|ActivateGlow (Variables|Default|GetTargetImage) 0.0)
        (Default|RegisterTriggerDeactivated (Variables|Default|GetConnectedCover))))))

(event EventBeginPlay)

(event Collision|EventActorBeginOverlap
  (params (OtherActor :type Actor%20Object%20Reference)))

(event EventTick
  (params (DeltaSeconds :type Float%20%28single-precision%29)))

(fn ConstructionScript)