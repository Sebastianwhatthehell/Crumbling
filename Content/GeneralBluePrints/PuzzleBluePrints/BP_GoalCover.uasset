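; BP_GoalCover is a puzzle cover that slides a hiding box open once enough triggers are active, and closes it when the count drops below the requirement.
; RegisterTriggerActivated and RegisterTriggerDeactivated maintain a count, clamped at zero on decrease, and compare it to the required count to call OpenCover or CloseCover.
; OpenCover plays a timeline that lerps the box along relative Y from its BeginPlay position, and CloseCover reverses it.
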(event Custom|OpenCover
  (bind _startlocation (Variables|Default|GetStartLocation))
  (bind (_x _y _z) (Math|Vector|BreakVector _startlocation))
  (bind _alpha (Timeline|TL_Move Play)
    (:Update
      (Transformation|SetRelativeLocation (Variables|Default|GetHidingBox) (Math|Vector|MakeVector _x (Math|Float|Lerp _y (+ (Variables|Default|GetMoveOffsetY) _y) _alpha) _z) false false))))

(event Custom|CloseCover
  (bind _startlocation (Variables|Default|GetStartLocation))
  (bind (_x _y _z) (Math|Vector|BreakVector _startlocation))
  (bind _alpha (Timeline|TL_Move Reverse)
    (:Update
      (Transformation|SetRelativeLocation (Variables|Default|GetHidingBox) (Math|Vector|MakeVector _x (Math|Float|Lerp _y (+ (Variables|Default|GetMoveOffsetY) _y) _alpha) _z) false false))))

(event EventBeginPlay
  (Variables|Default|SetStartLocation (Variables|/Script/Engine.SceneComponent|GetRelativeLocation (Variables|Default|GetHidingBox))))

(fn ConstructionScript)

(fn RegisterTriggerActivated
  (bind _currentcount (Variables|Default|GetCurrentCount))
  (Math|Integer|IncrementInt _currentcount
    (:%20%20
      (if (>= _currentcount (Variables|Default|GetRequiredCoun))
        (CallFunction|OpenCover)))))

(fn RegisterTriggerDeactivated
  (bind _result (Math|Integer|DecrementInt (Variables|Default|GetCurrentCount))
    (:%20%20
      (Variables|Default|SetCurrentCount (Math|Integer|Max(Integer) _result))
      (if (< (Variables|Default|GetCurrentCount) (Variables|Default|GetRequiredCoun))
        (CallFunction|CloseCover)))))