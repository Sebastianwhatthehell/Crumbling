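; BP_Tower is a tower actor whose tagged tile meshes drop by staggered amounts when TriggerFall fires.
; BeginPlay caches each "Tile" component's start transform and a drop height that grows with its index.
; The TL_Move timeline lerps tiles downward by scaling drop height with Alpha, teleporting them without sweep.
; Overlapping any of four recall triggers reverses the timeline, raising the tiles back toward their start positions.
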(event OnComponentBeginOverlap(RecallTrigger)
  (params (OverlappedComponent :type Primitive%20Component%20Object%20Reference) (OtherActor :type Actor%20Object%20Reference) (OtherComp :type Primitive%20Component%20Object%20Reference) (OtherBodyIndex :type Integer) (bFromSweep :type Boolean) (SweepResult :type Hit%20Result%20Structure%20%28by%20ref%29))
  (bind _alpha (Timeline|TL_Move Reverse)
    (:Update
      (for (_array_element _array_index) (Variables|Default|GetTiles)
        (Transformation|SetWorldLocation _array_element (Math|Vector|MakeVector (.X (Math|Vector|BreakVector (.Location (Math|Transform|BreakTransform (Utilities|Array|Get(acopy) (Variables|Default|GetStartTransforms) _array_index))))) (.Y (Math|Vector|BreakVector (.Location (Math|Transform|BreakTransform (Utilities|Array|Get(acopy) (Variables|Default|GetStartTransforms) _array_index))))) (- (.Z (Math|Vector|BreakVector (.Location (Math|Transform|BreakTransform (Utilities|Array|Get(acopy) (Variables|Default|GetStartTransforms) _array_index))))) (* (Utilities|Array|Get(acopy) (Variables|Default|GetDropHeights) _array_index) _alpha))) false true)))))

(event OnComponentBeginOverlap(RecallTrigger1)
  (params (OverlappedComponent :type Primitive%20Component%20Object%20Reference) (OtherActor :type Actor%20Object%20Reference) (OtherComp :type Primitive%20Component%20Object%20Reference) (OtherBodyIndex :type Integer) (bFromSweep :type Boolean) (SweepResult :type Hit%20Result%20Structure%20%28by%20ref%29))
  (bind _alpha (Timeline|TL_Move Reverse)
    (:Update
      (for (_array_element _array_index) (Variables|Default|GetTiles)
        (Transformation|SetWorldLocation _array_element (Math|Vector|MakeVector (.X (Math|Vector|BreakVector (.Location (Math|Transform|BreakTransform (Utilities|Array|Get(acopy) (Variables|Default|GetStartTransforms) _array_index))))) (.Y (Math|Vector|BreakVector (.Location (Math|Transform|BreakTransform (Utilities|Array|Get(acopy) (Variables|Default|GetStartTransforms) _array_index))))) (- (.Z (Math|Vector|BreakVector (.Location (Math|Transform|BreakTransform (Utilities|Array|Get(acopy) (Variables|Default|GetStartTransforms) _array_index))))) (* (Utilities|Array|Get(acopy) (Variables|Default|GetDropHeights) _array_index) _alpha))) false true)))))

(event OnComponentBeginOverlap(RecallTrigger2)
  (params (OverlappedComponent :type Primitive%20Component%20Object%20Reference) (OtherActor :type Actor%20Object%20Reference) (OtherComp :type Primitive%20Component%20Object%20Reference) (OtherBodyIndex :type Integer) (bFromSweep :type Boolean) (SweepResult :type Hit%20Result%20Structure%20%28by%20ref%29))
  (bind _alpha (Timeline|TL_Move Reverse)
    (:Update
      (for (_array_element _array_index) (Variables|Default|GetTiles)
        (Transformation|SetWorldLocation _array_element (Math|Vector|MakeVector (.X (Math|Vector|BreakVector (.Location (Math|Transform|BreakTransform (Utilities|Array|Get(acopy) (Variables|Default|GetStartTransforms) _array_index))))) (.Y (Math|Vector|BreakVector (.Location (Math|Transform|BreakTransform (Utilities|Array|Get(acopy) (Variables|Default|GetStartTransforms) _array_index))))) (- (.Z (Math|Vector|BreakVector (.Location (Math|Transform|BreakTransform (Utilities|Array|Get(acopy) (Variables|Default|GetStartTransforms) _array_index))))) (* (Utilities|Array|Get(acopy) (Variables|Default|GetDropHeights) _array_index) _alpha))) false true)))))

(event OnComponentBeginOverlap(RecallTrigger3)
  (params (OverlappedComponent :type Primitive%20Component%20Object%20Reference) (OtherActor :type Actor%20Object%20Reference) (OtherComp :type Primitive%20Component%20Object%20Reference) (OtherBodyIndex :type Integer) (bFromSweep :type Boolean) (SweepResult :type Hit%20Result%20Structure%20%28by%20ref%29))
  (bind _alpha (Timeline|TL_Move Reverse)
    (:Update
      (for (_array_element _array_index) (Variables|Default|GetTiles)
        (Transformation|SetWorldLocation _array_element (Math|Vector|MakeVector (.X (Math|Vector|BreakVector (.Location (Math|Transform|BreakTransform (Utilities|Array|Get(acopy) (Variables|Default|GetStartTransforms) _array_index))))) (.Y (Math|Vector|BreakVector (.Location (Math|Transform|BreakTransform (Utilities|Array|Get(acopy) (Variables|Default|GetStartTransforms) _array_index))))) (- (.Z (Math|Vector|BreakVector (.Location (Math|Transform|BreakTransform (Utilities|Array|Get(acopy) (Variables|Default|GetStartTransforms) _array_index))))) (* (Utilities|Array|Get(acopy) (Variables|Default|GetDropHeights) _array_index) _alpha))) false true)))))

(event EventBeginPlay
  (Variables|Default|SetPlayerRef (Game|GetPlayerCharacter 0))
  (for (_array_element _array_index) (Actor|GetComponentsbyTag "/Script/Engine.StaticMeshComponent" "Tile")
    (Utilities|Array|Add (Variables|Default|GetTiles) _array_element)
    (Utilities|Array|Add (Variables|Default|GetStartTransforms) (Transformation|GetWorldTransform _array_element))
    (Utilities|Array|Add (Variables|Default|GetDropHeights) (* (+ 1.0 (Math|Conversions|ToFloat(Integer) _array_index)) (Variables|Default|GetStepPerTile)))))

(event EventTriggerFall
  (bind _alpha (Timeline|TL_Move Play)
    (:Update
      (for (_array_element _array_index) (Variables|Default|GetTiles)
        (Transformation|SetWorldLocation _array_element (Math|Vector|MakeVector (.X (Math|Vector|BreakVector (.Location (Math|Transform|BreakTransform (Utilities|Array|Get(acopy) (Variables|Default|GetStartTransforms) _array_index))))) (.Y (Math|Vector|BreakVector (.Location (Math|Transform|BreakTransform (Utilities|Array|Get(acopy) (Variables|Default|GetStartTransforms) _array_index))))) (- (.Z (Math|Vector|BreakVector (.Location (Math|Transform|BreakTransform (Utilities|Array|Get(acopy) (Variables|Default|GetStartTransforms) _array_index))))) (* (Utilities|Array|Get(acopy) (Variables|Default|GetDropHeights) _array_index) _alpha))) false true)))))

(fn ConstructionScript)